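; BP_Cargo is a physics-driven cargo projectile that is meant to reach a specific destination planet.
; AddForce pushes its static mesh along the Arrow component's forward vector, scaling the input by MaximumForce.
; When the mesh hits any BP_Planets actor, it prints success or failure depending on whether that is DestinationPlanet, then spawns a particle effect and destroys itself.
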(event `self.ReceiveBeginPlay`)

(event `self.StaticMesh.OnComponentHit`
  (params (HitComponent :type "PrimitiveComponent Object Reference") (OtherActor :type "Actor Object Reference") (OtherComp :type "PrimitiveComponent Object Reference") (NormalImpulse :type "Vector Structure") (Hit :type "HitResult Structure (by ref)"))
  (bind (_returnvalue_location _returnvalue_rotation _returnvalue_scale) (`KismetMathLibrary.BreakTransform` (`self.GetTransform`)))
  (bind _asbp_planets (cast `/Game/Game/Blueprints/Planets/BP_Planets` OtherActor))
  (`|ExecutionSequence`
    (:`then_0`
      (if (== _asbp_planets (`self.DestinationPlanet`))
        (`KismetSystemLibrary.PrintString` "Success")
        (else
          (`KismetSystemLibrary.PrintString` "Failure"))))
    (:`then_1`
      (`GameplayStatics.SpawnEmitterAtLocation` "/Engine/Tutorial/SubEditors/TutorialAssets/TutorialParticleSystem.TutorialParticleSystem" _returnvalue_location (struct) _returnvalue_scale))
    (:`then_2`
      (`self.K2_DestroyActor`))))

(fn `AddForce`
  (params (Force :type "Float (double-precision)"))
  (locals (MaximumForce :type "Float (double-precision)" :default 1000000000.0))
  (`PrimitiveComponent.AddForce` (`self.StaticMesh`) (* (`SceneComponent.GetForwardVector` (`self.Arrow`)) (* Force (`local.MaximumForce`))) "None" false))

(fn `UserConstructionScript`)