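; BP_Cargo_Widget_Scene is a scene actor, apparently used for the cargo widget, that displays a static mesh with a gently swaying rotation.
; Each Tick sets the mesh's relative yaw to a sine of time since creation, scaled by speed and amplitude factors, so it oscillates back and forth rather than spinning.
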(event `self.ReceiveTick`
  (params (DeltaSeconds :type "Float (single-precision)"))
  (`SceneComponent.K2_SetRelativeRotation` (`self.StaticMesh`) (`KismetMathLibrary.MakeRotator` 0.0 0.0 (* (`KismetMathLibrary.DegSin` (* (`self.GetGameTimeSinceCreation`) (`self.RotationSpeedFactor`))) (`self.RotationFactor`))) false false))

(fn `UserConstructionScript`
  (`parent.UserConstructionScript`))