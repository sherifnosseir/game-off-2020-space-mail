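; BP_Planet is a planet actor that pulls overlapping actors toward itself, unless it is flagged as the home planet.
; Each Tick on a non-home planet passes the Sphere component to PullOverlappingActorsToPlanet, whose logic is defined outside this graph.
; The construction script scales Sphere from Scale, and sizes GravityPull from that scale plus GravitationSphereSize.
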(event `self.ReceiveTick`
  (params (DeltaSeconds :type "Float (single-precision)"))
  (if (not (`self.isHomePlanet`))
    (`self.PullOverlappingActorsToPlanet` (`self.Sphere`))))

(fn `UserConstructionScript`
  (bind _returnvalue (`KismetMathLibrary.Conv_DoubleToVector` (`self.Scale`)))
  (`SceneComponent.SetWorldScale3D` (`self.Sphere`) _returnvalue)
  (`SceneComponent.SetWorldScale3D` (`self.GravityPull`) (+ _returnvalue (`self.GravitationSphereSize`))))