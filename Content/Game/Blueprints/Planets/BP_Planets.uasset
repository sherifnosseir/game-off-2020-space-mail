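; BP_Planets is a planet actor that exerts gravity on nearby actors.
; Its construction script scales three spheres (planet, atmosphere, gravity) by cumulative size variables, so each outer radius builds on the inner ones.
; Every Tick, unless flagged as the home planet, it passes the gravity sphere and gravitational strength to PullOverlappingActorsToPlanet to attract overlapping actors.
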(event `self.ReceiveTick`
  (params (DeltaSeconds :type "Float (single-precision)"))
  (if (not (`self.isHomePlanet`))
    (`self.PullOverlappingActorsToPlanet` (`self.GravitySphere`) (`self.GravitationalStrength`))))

(fn `UserConstructionScript`
  (bind _planetsize (`self.PlanetSize`))
  (bind _atmospheresize (`self.AtmosphereSize`))
  (`|ExecutionSequence`
    (:`then_0`
      (`SceneComponent.SetWorldScale3D` (`self.PlanetSphere`) (`KismetMathLibrary.Conv_DoubleToVector` _planetsize)))
    (:`then_1`
      (`SceneComponent.SetWorldScale3D` (`self.AtmosphereSphere`) (`KismetMathLibrary.Conv_DoubleToVector` (+ _planetsize _atmospheresize))))
    (:`then_2`
      (`SceneComponent.SetWorldScale3D` (`self.GravitySphere`) (`KismetMathLibrary.Conv_DoubleToVector` (+ _planetsize _atmospheresize (`self.GravitySphereSize`)))))))