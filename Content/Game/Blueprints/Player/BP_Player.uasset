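; Player Blueprint for charging and launching cargo from an aiming gizmo around a planet, with a zoomable spring-arm camera.
; Holding Shoot builds clamped power shown on the game widget; release spawns BP_Cargo at the gizmo's marker and applies that force.
; The BP_PlayerGizmos actor receives move input, orients to the planet, and gets signed Shoot calls each tick through W/S gates.
; Scroll sets a zoom target that Tick lerps toward.
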(event `Key|W`
  (params (Key :type "Key Structure"))
  (:`Pressed`
    (goto _label :!via `Open`))
  (:`Released`
    (goto _label :!via `Close`)))

(event `Key|S`
  (params (Key :type "Key Structure"))
  (:`Pressed`
    (goto _label_2 :!via `Open`))
  (:`Released`
    (goto _label_2 :!via `Close`)))

(event `self.ReceiveBeginPlay`
  (set `self.DesiredZoom` (`SpringArmComponent.TargetArmLength` (`self.SpringArm`)))
  (bind _returnvalue (`|CreateWidget` "/Game/Game/Blueprints/Player/BP_GameWidget.BP_GameWidget_C"))
  (bind _output_get (set `self.AimWidget` _returnvalue))
  (`UserWidget.AddToViewport` _output_get 0)
  (bind _asbp_player_gizmos (cast `/Game/Game/Blueprints/Player/BP_PlayerGizmos` (`self.AimingActor`))
    (:`then`
      (set `self.AimingComponent` _asbp_player_gizmos))
    (:`CastFailed`
      (`KismetSystemLibrary.PrintString` "FAIOL"))))

(event `self.ReceiveTick`
  (params (DeltaSeconds :type "Float (single-precision)"))
  (`|ExecutionSequence`
    (:`then_0`
      (`self.UpdateCamera`))
    (:`then_1`
      (`self.HandleShoot`))
    (:`then_2`
      (`/Engine/EditorBlueprintResources/StandardMacros.Gate` true :!label _label
        (:`Exit`
          (`/Game/Game/Blueprints/Player/BP_PlayerGizmos.Shoot` (`self.AimingComponent`) -1.0))))
    (:`then_3`
      (`/Engine/EditorBlueprintResources/StandardMacros.Gate` true :!label _label_2
        (:`Exit`
          (`/Game/Game/Blueprints/Player/BP_PlayerGizmos.Shoot` (`self.AimingComponent`) 1.0))))))

(event `UpdateCamera`
  (bind _desiredzoom (`self.DesiredZoom`))
  (bind _targetarmlength (`SpringArmComponent.TargetArmLength` (`self.SpringArm`)))
  (if (!= _desiredzoom _targetarmlength)
    (set `SpringArmComponent.TargetArmLength` (`KismetMathLibrary.Lerp` _targetarmlength _desiredzoom (`self.ZoomRate`)) (`self.SpringArm`))))

(event `InputAxis|Scroll`
  (params (AxisValue :type "Float (single-precision)"))
  (bind _aimingcomponent (`self.AimingComponent`))
  (if (not (`KismetMathLibrary.NearlyEqual_FloatFloat` AxisValue 0.0 0.1))
    (set `self.DesiredZoom` (+ (* (`GameplayStatics.GetWorldDeltaSeconds`) (`self.ZoomSpeed`) AxisValue) (`SpringArmComponent.TargetArmLength` (`self.SpringArm`))))
    (`/Game/Game/Blueprints/Player/BP_PlayerGizmos.UpdateSpringArmDistance` _aimingcomponent (`KismetMathLibrary.Vector_Distance` (`SceneComponent.K2_GetComponentLocation` (`self.SpringArm`)) (`SceneComponent.K2_GetComponentLocation` (`/Game/Game/Blueprints/Player/BP_PlayerGizmos.SpringArm` _aimingcomponent))))))

(event `InputAction|Shoot`
  (params (Key :type "Key Structure"))
  (bind _aimingcomponent (`self.AimingComponent`))
  (bind _returnvalue (`SceneComponent.K2_GetComponentLocation` (`/Game/Game/Blueprints/Player/BP_PlayerGizmos.Widget` _aimingcomponent)))
  (bind _returnvalue_2 (`KismetMathLibrary.FindLookAtRotation` (`self.K2_GetActorLocation` _aimingcomponent) _returnvalue))
  (:`Pressed`
    (set `self.bIsShooting` true))
  (:`Released`
    (set `self.bIsShooting` false)
    (`KismetSystemLibrary.PrintString` (`KismetStringLibrary.Conv_RotatorToString` _returnvalue_2))
    (bind _returnvalue_3 (`|SpawnActorFromClass` "/Game/Game/Blueprints/BP_Cargo.BP_Cargo_C" (`KismetMathLibrary.MakeTransform` _returnvalue _returnvalue_2 (0.2 0.2 0.2)) "Undefined" "OverrideRootScale" null null))
    (`/Game/Game/Blueprints/BP_Cargo.AddForce` _returnvalue_3 (`self.CurrentPower`))
    (set `self.CurrentPower` 0.0)
    (set `/Game/Game/Blueprints/Player/BP_GameWidget.CurrentPower` (stale `HandleShoot` _output_get) (`self.AimWidget`) :!label _label_3)))

(event `HandleShoot`
  (if (`self.bIsShooting`)
    (bind _output_get (set `self.CurrentPower` (`KismetMathLibrary.FClamp` (+ (`self.CurrentPower`) (* (`self.PowerChangeRate`) (`GameplayStatics.GetWorldDeltaSeconds`))))))
    (goto _label_3)))

(event `InputAxis|MoveRight`
  (params (AxisValue :type "Float (single-precision)"))
  (bind _aimingcomponent (`self.AimingComponent`))
  (`/Game/Game/Blueprints/Player/BP_PlayerGizmos.Move` _aimingcomponent AxisValue)
  (`SceneComponent.K2_SetWorldRotation` (`Actor.RootComponent` _aimingcomponent) (`KismetMathLibrary.MakeRotator` (+ (.roll (`KismetMathLibrary.FindLookAtRotation` (`SceneComponent.K2_GetComponentLocation` (`/Game/Game/Blueprints/Player/BP_PlayerGizmos.DefaultSceneRoot` (`self.AimingComponent`))) (`self.K2_GetActorLocation` (`self.Planet`)))) 180.0) (+ (.pitch (`KismetMathLibrary.FindLookAtRotation` (`SceneComponent.K2_GetComponentLocation` (`/Game/Game/Blueprints/Player/BP_PlayerGizmos.DefaultSceneRoot` (`self.AimingComponent`))) (`self.K2_GetActorLocation` (`self.Planet`)))) -90.0) (.yaw (`KismetMathLibrary.FindLookAtRotation` (`SceneComponent.K2_GetComponentLocation` (`/Game/Game/Blueprints/Player/BP_PlayerGizmos.DefaultSceneRoot` (`self.AimingComponent`))) (`self.K2_GetActorLocation` (`self.Planet`))))) false false))

(fn `UserConstructionScript`)