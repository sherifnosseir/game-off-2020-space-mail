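; BP_PlayerGizmos is a player helper actor that exposes functions for moving itself and adjusting a spring arm for aiming.
; Move slides the root along its forward vector with sweep, and Shoot, despite its name, only pitches the spring arm, both scaled by axis input, rate and delta time.
; UpdateSpringArmDistance sets arm length from a distance divided by an aim factor.
; The event graph is empty, so nothing runs unless called externally.
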(fn `Move`
  (params (Axis :type "Float (double-precision)"))
  (bind _defaultsceneroot (`self.DefaultSceneRoot`))
  (`SceneComponent.K2_SetWorldLocation` _defaultsceneroot (+ (* (`SceneComponent.GetForwardVector` (`self.DefaultSceneRoot`)) (* Axis (`GameplayStatics.GetWorldDeltaSeconds`) (`self.MovementRate`))) (`SceneComponent.K2_GetComponentLocation` _defaultsceneroot)) true false))

(fn `Shoot`
  (params (Axis :type "Float (double-precision)"))
  (`SceneComponent.K2_AddLocalRotation` (`self.SpringArm`) (`KismetMathLibrary.MakeRotator` 0.0 (* Axis (`GameplayStatics.GetWorldDeltaSeconds`) (`self.AimTurnRate`))) false false))

(fn `UpdateSpringArmDistance`
  (params (Distance :type "Float (double-precision)"))
  (set `SpringArmComponent.TargetArmLength` (/ Distance (`self.AimDistanceFactor`)) (`self.SpringArm`)))

(fn `UserConstructionScript`)